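; Base enemy character Blueprint that provides sword combat, a patrol route and movement speed control.
; WieldSword spawns a BP_Sword, snaps it to the right-hand socket on the mesh and flags the sword as wielded.
; Attack plays the sword slash montage and fires the OnAttackEnd dispatcher whether it completes or is interrupted.
; GetPatrolRoute exposes the assigned route, and SetMovementSpeed maps a movement state to the walk speed and returns it.
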(event Custom|Attack
  (Animation|Montage|PlayMontage (Variables|Character|GetMesh) "/Game/_Game/Enemies/Animations/Melee/Montage_Sword_Slash.Montage_Sword_Slash"
    (:OnCompleted
      _)
    (:OnInterrupted
      _))
  (Default|CallOnAttackEnd))

(event Custom|WieldSword
  (bind _returnvalue (Game|SpawnActorfromClass "/Game/_Game/Weapons/BP_Sword.BP_Sword_C" (Transformation|GetActorTransform) "Undefined" "MultiplyWithRoot" 0 0))
  (Transformation|AttachComponentToComponent _returnvalue (Variables|Character|GetMesh) "hand_r_sword_socket" "SnapToTarget" "SnapToTarget" "SnapToTarget" true)
  (Variables|Default|SetbIsWieldingSword true))

(event EventBeginPlay)

(fn ConstructionScript)

(fn GetPatrolRoute
  (return (Variables|AI|GetPatrolRoute)))

(fn SetMovementSpeed
  (params (Speed :type E_MovementSpeed%20Enum :default "NewEnumerator0"))
  (bind _output_get (Variables|/Script/Engine.CharacterMovementComponent|SetMaxWalkSpeed (Variables|Character|GetCharacterMovement) (Utilities|Select :Index Speed :NewEnumerator0 0.0 :NewEnumerator1 1e+02 :NewEnumerator2 3e+02 :NewEnumerator3 5e+02)))
  (return _output_get))